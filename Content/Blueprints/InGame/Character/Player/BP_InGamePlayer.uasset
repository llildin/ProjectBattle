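; BP_InGamePlayer is the in-game player character Blueprint, whose only working logic here is a battle camera turn.
; BattleCameraSetting plays a Timeline that lerps the controller's control rotation from a start to an end rotator along the shortest path.
; Tick, TestAttackEvent_1 and the construction script are empty.
; Unwired debug leftovers would print the current state and sphere-trace for Pawns in front of the character.
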(event Custom|TestAttackEvent_1)

(event EventTick
  (params (DeltaSeconds :type Float%20%28single-precision%29)))

(event EventBattleCameraSetting
  (params (StartRotator :type Rotator :default "0, 0, 0") (EndRotator :type Rotator :default "0, 0, 0"))
  (bind _alpha (Timeline|Timeline PlayFromStart)
    (:Update
      (Pawn|SetControlRotation (Pawn|GetController) (Math|Rotator|Lerp(Rotator) StartRotator EndRotator _alpha true)))))

(fn ConstructionScript)